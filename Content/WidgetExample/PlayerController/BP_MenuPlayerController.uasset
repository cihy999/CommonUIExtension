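; BP_MenuPlayerController is a player controller that opens the main menu from an Enhanced Input action.
; BeginPlay adds the IMC_Menu mapping context with priority.
; When IA_OpenMenu completes, it lazily creates WB_MainMenu, caches it in MenuRef and adds it to the viewport.
; It then switches to Game and UI input focused on the menu and shows the mouse cursor, with no closing logic here.
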(event Input|EnhancedActionEvents|EnhancedInputActionIA_OpenMenu
  (params (ActionValue :type Boolean) (ElapsedSeconds :type Float%20%28double-precision%29) (TriggeredSeconds :type Float%20%28double-precision%29) (InputAction :type Input%20Action%20Object%20Reference :default "/Game/WidgetExample/PlayerController/IA_OpenMenu.IA_OpenMenu"))
  ;[1 1 1] Open Menu
  (:Completed
    (Utilities|IsValid (Variables|Default|GetMenuRef)
      (:Is%20Valid
        _)
      (:Is%20Not%20Valid
        (bind _returnvalue (UserInterface|CreateWidget "/Game/WidgetExample/WB_MainMenu.WB_MainMenu_C" self))
        (bind _output_get (Variables|Default|SetMenuRef _returnvalue))))
    (UserInterface|Viewport|AddtoViewport _output_get 0)
    (Input|SetInputModeGameandUI self _output_get "DoNotLock" true false)
    (Variables|Default|SetbShowMouseCursor true)))

(event EventBeginPlay
  (Input|AddMappingContext (PlayerController|LocalPlayerSubsystems|GetEnhancedInputLocalPlayerSubsystem) "/Game/WidgetExample/PlayerController/IMC_Menu.IMC_Menu" 1 "(bIgnoreAllPressedKeysUntilRelease=True,bForceImmediately=False,bNotifyUserSettings=False)"))

(fn ConstructionScript)